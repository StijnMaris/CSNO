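; BP_DummyTarget is a test dummy actor that visualizes incoming damage for debugging.
; Point damage draws a debug sphere and the damage value at the hit location, while radial damage prints its amount.
; Its CSNOHealth component's events print health changes with the damage causer and alive or died state, and death plays a non-looping animation on the skeletal mesh.
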(event `self.ReceivePointDamage`
  (params (Damage :type "Float (single-precision)") (DamageType :type "DamageType Object Reference") (HitLocation :type "Vector Structure") (HitNormal :type "Vector Structure") (HitComponent :type "PrimitiveComponent Object Reference") (BoneName :type Name) (ShotFromDirection :type "Vector Structure") (InstigatedBy :type "Controller Object Reference") (DamageCauser :type "Actor Object Reference") (HitInfo :type "HitResult Structure (by ref)"))
  (`KismetSystemLibrary.DrawDebugSphere` HitLocation 10.0 12 (struct :`R` 1.0 :`A` 1.0) 1.0 1.0)
  (`KismetSystemLibrary.DrawDebugString` HitLocation (`KismetStringLibrary.Conv_DoubleToString` Damage) null (struct :`R` 1.0 :`G` 1.0 :`B` 1.0 :`A` 1.0) 1.0))

(event `self.CSNOHealth.OnHealthChanged`
  (params (HealthComp :type "CSNOHealthComponent Object Reference") (Health :type "Float (single-precision)") (HealthDelta :type "Float (single-precision)") (DamageType :type "DamageType Object Reference") (InstigatedBy :type "Controller Object Reference") (DamageCauser :type "Actor Object Reference"))
  (`KismetSystemLibrary.PrintString` (`KismetStringLibrary.Concat_StrStr` (`KismetStringLibrary.Conv_DoubleToString` HealthDelta) (`KismetSystemLibrary.GetDisplayName` DamageCauser))))

(event `self.CSNOHealth.OnDied`
  (params (bIsDead :type Boolean) (VictimActor :type "Actor Object Reference") (KillerActor :type "Actor Object Reference") (KillerController :type "Controller Object Reference"))
  (if bIsDead
    (`KismetSystemLibrary.PrintString` "Died")
    (`SkeletalMeshComponent.PlayAnimation` (`self.SkeletalMesh`) "/Game/CSNO/Animations/Character/Death_1.Death_1" false)
    (else
      (`KismetSystemLibrary.PrintString` "Alive"))))

(event `self.ReceiveRadialDamage`
  (params (DamageReceived :type "Float (single-precision)") (DamageType :type "DamageType Object Reference") (Origin :type "Vector Structure") (HitInfo :type "HitResult Structure (by ref)") (InstigatedBy :type "Controller Object Reference") (DamageCauser :type "Actor Object Reference"))
  (`KismetSystemLibrary.PrintString` (`KismetStringLibrary.Concat_StrStr` (`KismetStringLibrary.Conv_DoubleToString` DamageReceived) " Radial Damage")))

(fn `UserConstructionScript`)