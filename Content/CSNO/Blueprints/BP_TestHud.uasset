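; BP_TestHud is a test HUD that puts the crosshair and main UI widgets on screen for the player's CSNO character.
; On BeginPlay it casts player 0's pawn and calls SetupWidgets, which creates both widgets and passes the pawn to WBP_UI.
; Tick polls that pawn and removes both widgets whenever it is invalid.
; The health component's death binding is disconnected and its OnDied handler is empty.
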(event `self.ReceiveBeginPlay`
  (bind _ascsnocharacter (cast `CSNOCharacter` (`GameplayStatics.GetPlayerPawn` 0)))
  (`self.SetupWidgets` _ascsnocharacter))

(event `OnDied`
  (params (bIsDead :type Boolean) (VictimActor :type "Actor Object Reference") (KillerActor :type "Actor Object Reference") (KillerController :type "Controller Object Reference")))

(event `self.ReceiveTick`
  (params (DeltaSeconds :type "Float (single-precision)"))
  (`/Engine/EditorBlueprintResources/StandardMacros.IsValid` (`GameplayStatics.GetPlayerPawn` 0)
    (:`Is Not Valid`
      (`Widget.RemoveFromParent` (`self.CrossHairWidget`))
      (`Widget.RemoveFromParent` (`self.UIWidget`)))))

(fn `SetupWidgets`
  (params (PawnReference :type "CSNOCharacter Object Reference"))
  (bind _returnvalue (`|CreateWidget` "/Game/CSNO/UI/WBP_Crosshair.WBP_Crosshair_C"))
  (bind _output_get (set `self.CrossHairWidget` _returnvalue))
  (`UserWidget.AddToViewport` _output_get 0)
  (bind _returnvalue_2 (`|CreateWidget` "/Game/CSNO/Blueprints/WBP_UI.WBP_UI_C"))
  (set `/Game/CSNO/Blueprints/WBP_UI.PawnReference` PawnReference _returnvalue_2)
  (bind _output_get_2 (set `self.UIWidget` _returnvalue_2))
  (`UserWidget.AddToViewport` _output_get_2 0))

(fn `UserConstructionScript`)