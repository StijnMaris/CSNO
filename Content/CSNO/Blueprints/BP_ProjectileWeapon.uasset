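; BP_ProjectileWeapon is a weapon actor that predicts a projectile path every frame, with no firing logic in the graph.
; BeginPlay casts the owner to CSNOCharacter and caches it as Player.
; Tick aims from the actor's location toward a point far along the player's view, using that offset as launch velocity.
; The collision-traced prediction ignores the player, and its results are unused.
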(event `self.ReceiveBeginPlay`
  (bind _ascsnocharacter (cast `CSNOCharacter` (`self.GetOwner`)))
  (set `self.Player` _ascsnocharacter))

(event `self.ReceiveTick`
  (params (DeltaSeconds :type "Float (single-precision)"))
  (bind _returnvalue (`self.K2_GetActorLocation`))
  (bind _player (`self.Player`))
  (bind (_outlocation _outrotation) (`self.GetActorEyesViewPoint` _player))
  (`GameplayStatics.Blueprint_PredictProjectilePath_Advanced` (make `PredictProjectilePathParams` :`StartLocation` _returnvalue :`LaunchVelocity` (- (+ _outlocation (* (`KismetMathLibrary.Conv_RotatorToVector` _outrotation) 3000)) _returnvalue) :`bTraceWithCollision` true :`ProjectileRadius` 5.0 :`ActorsToIgnore` (`|MakeArray` _player :!type "Actor Object Reference") :`SimFrequency` 100.0)))

(fn `UserConstructionScript`)