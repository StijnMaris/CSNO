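; BP_DamageZone is an area hazard that repeatedly damages actors around its location.
; On BeginPlay, a Damage event applies radial damage at full strength within DamageRadius, ignoring itself and crediting its instigator and that instigator's controller.
; The event then waits DamageInterval and calls itself again, looping with no stop condition in the graph rather than relying on overlap or Tick.
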(event `self.ReceiveBeginPlay`
  (`self.Damage`))

(event `self.ReceiveTick`
  (params (DeltaSeconds :type "Float (single-precision)")))

(event `Damage`
  (`GameplayStatics.ApplyRadialDamage` (`self.BaseDamage`) (`self.K2_GetActorLocation`) (`self.DamageRadius`) null (`|MakeArray` self :!type "Actor Object Reference") (`self.GetInstigator`) (`self.GetInstigatorController`) true)
  (`KismetSystemLibrary.Delay` (`self.DamageInterval`))
  (`self.Damage`))

(fn `UserConstructionScript`)