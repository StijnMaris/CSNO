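; Flashbang projectile Blueprint that blinds the local player with a white screen and audio fade when it explodes.
; After the parent explosion, the non-authority side finds the locally controlled CSNOCharacter and line-traces to its first-person camera on Visibility.
; If the trace hits a character, fade duration scales with the dot product of camera forward and direction to the grenade, so facing it blinds longer.
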(event `self.Explode`
  (bind _returnvalue (`self.K2_GetActorLocation`))
  (`parent.Explode`)
  (`/Engine/EditorBlueprintResources/ActorMacros.Switch Has Authority`
    (:`Remote`
      (bind _outactors (`GameplayStatics.GetAllActorsOfClass` "/Script/CSNO.CSNOCharacter"))
      (for _array_element _outactors
        (if (`Pawn.IsLocallyControlled` _array_element)
          (bind _firstpersoncameracomponent (`CSNOCharacter.FirstPersonCameraComponent` _array_element))
          (bind _returnvalue_2 (`SceneComponent.K2_GetComponentLocation` _firstpersoncameracomponent))
          (bind _outhit (`KismetSystemLibrary.LineTraceSingle` _returnvalue _returnvalue_2 "TraceTypeQuery1" false (`|MakeArray` self :!type "Actor Object Reference")))
          (cast `CSNOCharacter` (`.HitActor` (`GameplayStatics.BreakHitResult` _outhit)))
          (`PlayerCameraManager.StartCameraFade` (`GameplayStatics.GetPlayerCameraManager` 0) 1.0 0.0 (* (`KismetMathLibrary.NormalizeToRange` (`KismetMathLibrary.Dot_VectorVector` (`SceneComponent.GetForwardVector` _firstpersoncameracomponent) (`KismetMathLibrary.GetForwardVector` (`KismetMathLibrary.FindLookAtRotation` _returnvalue_2 _returnvalue))) -0.9 1.0) 5.0) (struct :`R` 1.0 :`G` 1.0 :`B` 1.0 :`A` 1.0) true false))))))

(fn `UserConstructionScript`)